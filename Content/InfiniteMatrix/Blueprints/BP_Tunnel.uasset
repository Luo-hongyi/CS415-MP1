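; Tunnel segment with a rotating holed wall, health and energy pickups, and an enemy.
; Randomize functions vary the hole mesh, roll and item offsets, and drop each pickup at random.
; Passing the trigger makes TunnelSpawner spawn another tunnel, destroys this one, and rewards score and energy, unless the wall was hit.
; Wall and enemy hits damage the player and can trigger restart, while shooting the enemy rewards the bullet's shooter.
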(event `self.ReceiveTick`
  (params (DeltaSeconds :type "Float (single-precision)"))
  (`SceneComponent.K2_AddLocalRotation` (`self.WallMesh`) (`KismetMathLibrary.MakeRotator` (* DeltaSeconds (`self.RotateSpeed`))) false false))

(event `self.TriggerZone.OnComponentBeginOverlap`
  (params (OverlappedComponent :type "PrimitiveComponent Object Reference") (OtherActor :type "Actor Object Reference") (OtherComp :type "PrimitiveComponent Object Reference") (OtherBodyIndex :type Integer) (bFromSweep :type Boolean) (SweepResult :type "HitResult Structure (by ref)"))
  (bind _asbp_player (cast `/Game/InfiniteMatrix/Blueprints/BP_Player` OtherActor))
  (`/Game/InfiniteMatrix/Blueprints/BP_TunnelSpawner.SpawnTunnelAtSpawnPoint` (`self.TunnelSpawner`))
  (`self.K2_DestroyActor`)
  (if (not (`self.HitWall`))
    (bind _current_score (`/Game/InfiniteMatrix/Blueprints/BP_Player.ChangeScore` _asbp_player 20))
    (`/Game/InfiniteMatrix/UI/ScoreText.Update Score Text` (`/Game/InfiniteMatrix/Blueprints/BP_Player.WB Score Text` _asbp_player) _current_score)
    (set `self.HitWall` false)
    (`/Game/InfiniteMatrix/Blueprints/BP_Player.ChangeEnergy` _asbp_player 5.0)))

(event `self.WallMesh.OnComponentBeginOverlap`
  (params (OverlappedComponent :type "PrimitiveComponent Object Reference") (OtherActor :type "Actor Object Reference") (OtherComp :type "PrimitiveComponent Object Reference") (OtherBodyIndex :type Integer) (bFromSweep :type Boolean) (SweepResult :type "HitResult Structure (by ref)"))
  (bind _asbp_player (cast `/Game/InfiniteMatrix/Blueprints/BP_Player` OtherActor)
    (:`then`
      (bind _current_health (`/Game/InfiniteMatrix/Blueprints/BP_Player.ChangeHealth` _asbp_player -20.0))
      (set `self.HitWall` true)
      (if (<= _current_health 0.0)
        (set `/Game/InfiniteMatrix/Blueprints/BP_Player.IsDead` true _asbp_player)
        (`/Game/InfiniteMatrix/Blueprints/BP_Player.DisplayRestart` _asbp_player)
        (elif (`/Game/InfiniteMatrix/Blueprints/BP_Player.Immune` _asbp_player)
          (`/Game/InfiniteMatrix/Blueprints/BP_Player.ChangeScore` _asbp_player 20))))
    (:`CastFailed`
      (bind _asbulet (cast `/Game/InfiniteMatrix/Blueprints/Bulet` OtherActor))
      (`self.K2_DestroyActor` _asbulet))))

(event `self.HealthKit.OnComponentBeginOverlap`
  (params (OverlappedComponent :type "PrimitiveComponent Object Reference") (OtherActor :type "Actor Object Reference") (OtherComp :type "PrimitiveComponent Object Reference") (OtherBodyIndex :type Integer) (bFromSweep :type Boolean) (SweepResult :type "HitResult Structure (by ref)"))
  (bind _asbp_player (cast `/Game/InfiniteMatrix/Blueprints/BP_Player` OtherActor))
  (`/Game/InfiniteMatrix/Blueprints/BP_Player.ChangeHealth` _asbp_player 10.0)
  (`ActorComponent.K2_DestroyComponent` (`self.HealthKit`)))

(event `self.EnergyPack.OnComponentBeginOverlap`
  (params (OverlappedComponent :type "PrimitiveComponent Object Reference") (OtherActor :type "Actor Object Reference") (OtherComp :type "PrimitiveComponent Object Reference") (OtherBodyIndex :type Integer) (bFromSweep :type Boolean) (SweepResult :type "HitResult Structure (by ref)"))
  (bind _asbp_player (cast `/Game/InfiniteMatrix/Blueprints/BP_Player` OtherActor))
  (`/Game/InfiniteMatrix/Blueprints/BP_Player.ChangeEnergy` _asbp_player 40.0)
  (`ActorComponent.K2_DestroyComponent` (`self.EnergyPack`)))

(event `self.Enemy.OnComponentBeginOverlap`
  (params (OverlappedComponent :type "PrimitiveComponent Object Reference") (OtherActor :type "Actor Object Reference") (OtherComp :type "PrimitiveComponent Object Reference") (OtherBodyIndex :type Integer) (bFromSweep :type Boolean) (SweepResult :type "HitResult Structure (by ref)"))
  (bind _asbp_player (cast `/Game/InfiniteMatrix/Blueprints/BP_Player` OtherActor)
    (:`then`
      (bind _current_health (`/Game/InfiniteMatrix/Blueprints/BP_Player.ChangeHealth` _asbp_player -20.0))
      (if (> _current_health 0.0)
        (`ActorComponent.K2_DestroyComponent` (`self.Enemy`))
        (else
          (set `/Game/InfiniteMatrix/Blueprints/BP_Player.IsDead` true _asbp_player)
          (`/Game/InfiniteMatrix/Blueprints/BP_Player.DisplayRestart` _asbp_player))))
    (:`CastFailed`
      (bind _asbulet (cast `/Game/InfiniteMatrix/Blueprints/Bulet` OtherActor))
      (if (`KismetSystemLibrary.IsValid` _asbulet)
        (`|ExecutionSequence`
          (:`then_0`
            (bind _shooter (`/Game/InfiniteMatrix/Blueprints/Bulet.Get Shooter` _asbulet))
            (`/Game/InfiniteMatrix/Blueprints/BP_Player.ChangeEnergy` _shooter 10.0))
          (:`then_1`
            (bind _shooter_2 (`/Game/InfiniteMatrix/Blueprints/Bulet.Get Shooter` _asbulet))
            (`/Game/InfiniteMatrix/Blueprints/BP_Player.ChangeScore` _shooter_2 20))
          (:`then_2`
            (bind _shooter_3 (`/Game/InfiniteMatrix/Blueprints/Bulet.Get Shooter` _asbulet))
            (`/Game/InfiniteMatrix/Blueprints/BP_Player.ChangeHealth` _shooter_3 10.0))
          (:`then_3`
            (`KismetSystemLibrary.Delay` 0.001)
            (`self.K2_DestroyActor` _asbulet))
          (:`then_4`
            (`ActorComponent.K2_DestroyComponent` (`self.Enemy`))))))))

(fn `RandomizeEnemy`
  (`SceneComponent.K2_AddWorldOffset` (`self.Enemy`) (`KismetMathLibrary.MakeVector` (`KismetMathLibrary.RandomFloatInRange` -200.0 200.0) (`KismetMathLibrary.RandomFloatInRange` -200.0 200.0) (`KismetMathLibrary.RandomFloatInRange` -200.0 200.0)) false false))

(fn `RandomizeEnergyPack`
  (bind _energypack (`self.EnergyPack`))
  (if (>= (`KismetMathLibrary.RandomIntegerInRange` 0 9) 3)
    (`ActorComponent.K2_DestroyComponent` _energypack)
    (else
      (`SceneComponent.K2_AddWorldOffset` _energypack (`KismetMathLibrary.MakeVector` (`KismetMathLibrary.RandomFloatInRange` -100.0 100.0) (`KismetMathLibrary.RandomFloatInRange` -100.0 100.0) (`KismetMathLibrary.RandomFloatInRange` -100.0 100.0)) false false))))

(fn `RandomizeHealthKit`
  (bind _healthkit (`self.HealthKit`))
  (if (>= (`KismetMathLibrary.RandomIntegerInRange` 0 9) 3)
    (`ActorComponent.K2_DestroyComponent` _healthkit)
    (else
      (`SceneComponent.K2_AddWorldOffset` _healthkit (`KismetMathLibrary.MakeVector` (`KismetMathLibrary.RandomFloatInRange` -100.0 100.0) (`KismetMathLibrary.RandomFloatInRange` -100.0 100.0) (`KismetMathLibrary.RandomFloatInRange` -100.0 100.0)) false false))))

(fn `RandomizeWall`
  (`StaticMeshComponent.SetStaticMesh` (`self.WallMesh`) (select `int` (`KismetMathLibrary.RandomIntegerInRange` 0 3) :`0` "/Game/InfiniteMatrix/Meshes/SM_Hole_01.SM_Hole_01" :`1` "/Game/InfiniteMatrix/Meshes/SM_Hole_02.SM_Hole_02" :`2` "/Game/InfiniteMatrix/Meshes/SM_Hole_03.SM_Hole_03" :`3` "/Game/InfiniteMatrix/Meshes/SM_Hole_04.SM_Hole_04" :!type "StaticMesh Object Reference"))
  (`SceneComponent.K2_AddLocalRotation` (`self.WallMesh`) (`KismetMathLibrary.MakeRotator` (`KismetMathLibrary.RandomFloatInRange` 0.0 360.0)) false false))

(fn `UserConstructionScript`)